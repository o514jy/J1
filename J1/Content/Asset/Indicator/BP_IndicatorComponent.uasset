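; Actor component that displays ability indicators on its owner: radius, cone and line shapes for casting or preview, plus range and target markers.
; Each event lazily spawns one of three BP_Indicator actors (main, range, target), attaches it to the owner, then forwards the call with the shared IndicatorHeight.
; Server-prefixed events drive timed casts on the main indicator, which Interrupt cancels.
; ShowTarget&Range combines both markers, using the range radius as the target's max range.
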(event `Server_CastRadius`
  (params (CastingTime :type "Float (double-precision)") (Alignement :type "/Game/RPG_Indicator/Data/Enumerator/E_Alignement Enum" :default "NewEnumerator0") (Radius :type "Float (double-precision)") (`Follow Type` :type "/Game/RPG_Indicator/Data/Enumerator/E_FollowType Enum" :default "NewEnumerator0") (Range :type "Float (double-precision)"))
  ;[0.1844 0.1844 0.1844] Cast Indicator
  (`self.Create Indicator?`)
  (`/Game/RPG_Indicator/Blueprint/BP_Indicator.CastRadius` (`self.Indicator`) CastingTime Alignement (`self.IndicatorHeight`) Radius `Follow Type` Range))

(event `ShowRadius`
  (params (Radius :type "Float (double-precision)") (ShowIndicator :type Boolean) (`Follow Type` :type "/Game/RPG_Indicator/Data/Enumerator/E_FollowType Enum" :default "NewEnumerator0") (`Max Range` :type "Float (double-precision)"))
  ;[0.1844 0.1844 0.1844] Show Indicator
  (`self.Create Indicator?`)
  (`/Game/RPG_Indicator/Blueprint/BP_Indicator.ShowRadius` (`self.Indicator`) (`self.IndicatorHeight`) Radius ShowIndicator `Follow Type` `Max Range`))

(event `Server_Cast Cone`
  (params (CastingTime :type "Float (double-precision)") (Alignement :type "/Game/RPG_Indicator/Data/Enumerator/E_Alignement Enum" :default "NewEnumerator0") (Range :type "Float (double-precision)") (Angle :type "Float (double-precision)") (TargetType :type "/Game/RPG_Indicator/Data/Enumerator/E_RotateType Enum" :default "NewEnumerator0"))
  ;[0.1844 0.1844 0.1844] Cast Indicator
  (`self.Create Indicator?`)
  (`/Game/RPG_Indicator/Blueprint/BP_Indicator.CastCone` (`self.Indicator`) CastingTime Alignement (`self.IndicatorHeight`) Range Angle TargetType))

(event `ShowCone`
  (params (TargetType :type "/Game/RPG_Indicator/Data/Enumerator/E_RotateType Enum" :default "NewEnumerator0") (Range :type "Float (double-precision)") (Angle :type "Float (double-precision)") (ShowIndicator :type Boolean))
  ;[0.1844 0.1844 0.1844] Show Indicator
  (`self.Create Indicator?`)
  (`/Game/RPG_Indicator/Blueprint/BP_Indicator.ShowCone` (`self.Indicator`) TargetType (`self.IndicatorHeight`) Range Angle ShowIndicator))

(event `Server_Cast Line`
  (params (CastingTime :type "Float (double-precision)") (Alignement :type "/Game/RPG_Indicator/Data/Enumerator/E_Alignement Enum" :default "NewEnumerator0") (Length :type "Float (double-precision)") (TargetType :type "/Game/RPG_Indicator/Data/Enumerator/E_RotateType Enum" :default "NewEnumerator0"))
  ;[0.1844 0.1844 0.1844] Cast Indicator
  (`self.Create Indicator?`)
  (`/Game/RPG_Indicator/Blueprint/BP_Indicator.CastLine` (`self.Indicator`) CastingTime Alignement (`self.IndicatorHeight`) Length TargetType))

(event `ShowLine`
  (params (`Target Type` :type "/Game/RPG_Indicator/Data/Enumerator/E_RotateType Enum" :default "NewEnumerator0") (Length :type "Float (double-precision)") (ShowIndicator :type Boolean))
  ;[0.1844 0.1844 0.1844] Show Indicator
  (`self.Create Indicator?`)
  (`/Game/RPG_Indicator/Blueprint/BP_Indicator.ShowLine` (`self.Indicator`) `Target Type` (`self.IndicatorHeight`) Length ShowIndicator))

(event `Show Range`
  (params (Radius :type "Float (double-precision)") (`bShowIndicator?` :type Boolean))
  ;[0.1844 0.1844 0.1844] Show Indicator
  (`self.Create Range Indicator?`)
  (`/Game/RPG_Indicator/Blueprint/BP_Indicator.ShowRange` (`self.RangeIndicator`) (`self.IndicatorHeight`) Radius `bShowIndicator?`))

(event `Show Target`
  (params (Radius :type "Float (double-precision)") (MaxRange :type "Float (double-precision)") (`bShowIndicator?` :type Boolean) (FollowType :type "/Game/RPG_Indicator/Data/Enumerator/E_FollowType Enum" :default "NewEnumerator0"))
  ;[0.1844 0.1844 0.1844] Show Indicator
  (`self.Create Target Indicator?`)
  (`/Game/RPG_Indicator/Blueprint/BP_Indicator.ShowTarget` (`self.TargetIndicator`) (`self.IndicatorHeight`) Radius MaxRange `bShowIndicator?` FollowType))

(event `Server_Interrupt`
  ;[0.1844 0.1844 0.1844] Interrupt
  (`self.Interrupt`))

(event `Interrupt`
  ;[0.1844 0.1844 0.1844] Interrupt
  (`/Game/RPG_Indicator/Blueprint/BP_Indicator.Interrupt` (`self.Indicator`)))

(event `Show Target&Range`
  (params (`Range Radius` :type "Float (double-precision)") (`Target Radius` :type "Float (double-precision)") (`bShowIndicator?` :type Boolean) (FollowType :type "/Game/RPG_Indicator/Data/Enumerator/E_FollowType Enum" :default "NewEnumerator0"))
  ;[0.1844 0.1844 0.1844] Show Indicator
  (`|ExecutionSequence`
    (:`then_0`
      (`self.Create Range Indicator?`)
      (`/Game/RPG_Indicator/Blueprint/BP_Indicator.ShowRange` (`self.RangeIndicator`) (`self.IndicatorHeight`) `Range Radius` `bShowIndicator?`))
    (:`then_1`
      (`self.Create Target Indicator?`)
      (`/Game/RPG_Indicator/Blueprint/BP_Indicator.ShowTarget` (`self.TargetIndicator`) (`self.IndicatorHeight`) `Target Radius` `Range Radius` `bShowIndicator?` FollowType))))

(fn `Create Indicator?`
  (bind _returnvalue (`self.GetOwner`))
  (`/Engine/EditorBlueprintResources/StandardMacros.IsValid` (`self.Indicator`)
    (:`Is Valid`
      _)
    (:`Is Not Valid`
      (bind _returnvalue_2 (`|SpawnActorFromClass` "/Game/RPG_Indicator/Blueprint/BP_Indicator.BP_Indicator_C" (`KismetMathLibrary.MakeTransform` (0.0 0.0 -90.0)) "AlwaysSpawn" "MultiplyWithRoot" _returnvalue null))
      (set `self.Indicator` _returnvalue_2)
      (set `self.IndicatorDecal` (`Actor.RootComponent` _returnvalue_2))
      (`Actor.K2_AttachToActor` _returnvalue_2 _returnvalue "None" "SnapToTarget" "KeepWorld" "KeepWorld" false)))
  (return))

(fn `Create Range Indicator?`
  (bind _returnvalue (`self.GetOwner`))
  (`/Engine/EditorBlueprintResources/StandardMacros.IsValid` (`self.RangeIndicator`)
    (:`Is Valid`
      _)
    (:`Is Not Valid`
      (bind _returnvalue_2 (`|SpawnActorFromClass` "/Game/RPG_Indicator/Blueprint/BP_Indicator.BP_Indicator_C" (`KismetMathLibrary.MakeTransform` (0.0 0.0 -90.0)) "AlwaysSpawn" "MultiplyWithRoot" _returnvalue null))
      (set `self.RangeIndicator` _returnvalue_2)
      (set `self.RangeDecal` (`Actor.RootComponent` _returnvalue_2))
      (`Actor.K2_AttachToActor` _returnvalue_2 _returnvalue "None" "SnapToTarget" "KeepWorld" "KeepWorld" false)))
  (return))

(fn `Create Target Indicator?`
  (bind _returnvalue (`self.GetOwner`))
  (`/Engine/EditorBlueprintResources/StandardMacros.IsValid` (`self.TargetIndicator`)
    (:`Is Valid`
      _)
    (:`Is Not Valid`
      (bind _returnvalue_2 (`|SpawnActorFromClass` "/Game/RPG_Indicator/Blueprint/BP_Indicator.BP_Indicator_C" (`KismetMathLibrary.MakeTransform` (0.0 0.0 -90.0)) "AlwaysSpawn" "MultiplyWithRoot" _returnvalue null))
      (set `self.TargetIndicator` _returnvalue_2)
      (set `self.TargetDecal` (`Actor.RootComponent` _returnvalue_2))
      (`Actor.K2_AttachToActor` _returnvalue_2 _returnvalue "None" "SnapToTarget" "KeepWorld" "KeepWorld" false)))
  (return))